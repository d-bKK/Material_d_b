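; BP_MeshRotater is an actor that spins a configurable static mesh around its vertical axis.
; The construction script applies the chosen mesh and its first material to the component.
; On BeginPlay, a timeline drives the world yaw each update with pitch and roll held at zero, and restarts when finished if Loop is set.
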(event EventBeginPlay
  (bind _新建轨道_0 (Timeline|时间轴 Play)
    (:Update
      (Transformation|SetWorldRotation (Variables|Default|GetStaticMesh) (Math|Rotator|MakeRotator 0.0 0.0 _新建轨道_0) false false))
    (:Finished
      (if (Variables|Public|GetLoop?)
        (Timeline|时间轴 PlayFromStart)))))

(fn ConstructionScript
  (bind _staticmesh (Variables|Default|GetStaticMesh))
  (Components|StaticMesh|SetStaticMesh _staticmesh (Variables|Public|GetNew%20Mesh))
  (Rendering|Material|SetMaterial _staticmesh 0 (Variables|Public|GetMaterial_0)))